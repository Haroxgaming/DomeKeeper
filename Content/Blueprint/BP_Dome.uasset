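; BP_Dome is a dome actor that slides a Cube along an elliptical arc to track the Plane component of BP_Camera.
; The construction script derives the arc's Y and Z radii from the Sphere's scale and sets the Cube's initial relative transform.
; Each tick, RotateCube rolls by the arctangent of its Y/Z offset to that Plane.
; That roll, clamped to ±90°, sets the Cube's world Y/Z via sine and cosine, without an actor-origin offset.
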(event `self.ReceiveBeginPlay`
  (bind _returnvalue (`GameplayStatics.GetActorOfClass` "/Game/Blueprint/BP_Camera.BP_Camera_C"))
  (set `self.Player ref` _returnvalue))

(event `self.ReceiveTick`
  (params (DeltaSeconds :type "Float (single-precision)"))
  (bind _cube (`self.Cube`))
  (bind _returnvalue_x (`KismetMathLibrary.BreakVector` (`SceneComponent.K2_GetComponentLocation` _cube)))
  (bind (_returnvalue_x_2 _returnvalue_y _returnvalue_z) (`KismetMathLibrary.BreakVector` (`SceneComponent.K2_GetComponentLocation` (`self.RotateCube`))))
  (bind _returnvalue_roll (`KismetMathLibrary.BreakRotator` (`SceneComponent.K2_GetComponentRotation` (`self.RotateCube`))))
  (bind _returnvalue (`KismetMathLibrary.FClamp` _returnvalue_roll -90.0 90.0))
  (bind (_returnvalue_x_3 _returnvalue_y_2 _returnvalue_z_2) (`KismetMathLibrary.BreakVector` (`SceneComponent.K2_GetComponentLocation` (`/Game/Blueprint/BP_Camera.Plane` (`self.Player ref`)))))
  (`SceneComponent.K2_SetWorldRotation` (`self.RotateCube`) (`KismetMathLibrary.MakeRotator` (`KismetMathLibrary.DegAtan` (/ (- _returnvalue_y_2 _returnvalue_y) (- _returnvalue_z_2 _returnvalue_z)))) false false)
  (`SceneComponent.K2_SetWorldLocation` _cube (`KismetMathLibrary.MakeVector` _returnvalue_x (* (`KismetMathLibrary.DegSin` _returnvalue) (`self.Longueur`)) (* (`KismetMathLibrary.DegCos` _returnvalue) (`self.Hauteur`))) false false))

(fn `UserConstructionScript`
  (bind _cube (`self.Cube`))
  (bind _returnvalue_x (`KismetMathLibrary.BreakVector` (`SceneComponent.K2_GetComponentLocation` _cube)))
  (bind _returnvalue_roll (`KismetMathLibrary.BreakRotator` (`SceneComponent.K2_GetComponentRotation` (`self.RotateCube`))))
  (bind (_returnvalue_x_2 _returnvalue_y _returnvalue_z) (`KismetMathLibrary.BreakVector` (`SceneComponent.K2_GetComponentScale` (`self.Sphere`))))
  (bind _returnvalue (`KismetMathLibrary.FClamp` _returnvalue_roll -90.0 90.0))
  (set `self.Longueur` (* _returnvalue_y 50.0))
  (set `self.Hauteur` (* _returnvalue_z 50.0))
  (`SceneComponent.K2_SetRelativeLocation` _cube (`KismetMathLibrary.MakeVector` _returnvalue_x (* (`KismetMathLibrary.DegSin` _returnvalue) (`self.Longueur`)) (* (`KismetMathLibrary.DegCos` _returnvalue) (`self.Hauteur`))) false false)
  (`SceneComponent.K2_SetRelativeRotation` _cube (`KismetMathLibrary.MakeRotator` _returnvalue) false false))